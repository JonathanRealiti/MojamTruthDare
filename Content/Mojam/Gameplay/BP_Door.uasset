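; BP_Door is a hinged door that swings open when it receives an Interact event.
; Interact plays a squeak sound and runs the OpenDoor timeline, which lerps the Door's relative yaw through a quarter turn.
; When the timeline finishes, a delay starts, after which the door squeaks again and reverses the timeline to close itself automatically.
; An IsOpen flag ignores interactions while the door is open.
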(event EventBeginPlay)

(event Collision|EventActorBeginOverlap
  (params (OtherActor :type Actor%20Object%20Reference)))

(event EventTick
  (params (DeltaSeconds :type Float%20%28single-precision%29)))

(event EventInteract
  (if (not (Variables|Default|GetIsOpen))
    (Variables|Default|SetIsOpen true)
    (Audio|PlaySoundatLocation "/Game/Mojam/Sound/Cue_SqueakSlower.Cue_SqueakSlower" (Transformation|GetActorLocation))
    (bind _dooropenratio (Timeline|OpenDoor Play)
      (:Update
        (Transformation|SetRelativeRotation (Variables|Default|GetDoor) (Math|Rotator|Lerp(Rotator) (Math|Rotator|MakeRotator 0.0 0.0 -1.8e+02) (Math|Rotator|MakeRotator 0.0 0.0 -9e+01) _dooropenratio true) false false))
      (:Finished
        (Utilities|FlowControl|Delay 5.0)
        (if (Variables|Default|GetIsOpen)
          (Variables|Default|SetIsOpen false)
          (Audio|PlaySoundatLocation "/Game/Mojam/Sound/Cue_SqueakSlower.Cue_SqueakSlower" (Transformation|GetActorLocation))
          (Utilities|String|Reverse (Variables|Default|GetOpenDoor)))))))

(fn ConstructionScript)